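; BP_InteractableDoor is a door actor that swings open when interacted with and closes when the player character leaves its interaction box.
; Interact, if the door is not open, scales a timeline's play rate by TimeToOpenS and plays it, lerping the mesh's yaw between closed and open positions.
; End overlap by MazeGamePlayerCharacter reverses the same timeline, whose Finished output toggles IsOpen in either direction.
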(event OnComponentEndOverlap(Box_Interaction)
  (params (OverlappedComponent :type Primitive%20Component%20Object%20Reference) (OtherActor :type Actor%20Object%20Reference) (OtherComp :type Primitive%20Component%20Object%20Reference) (OtherBodyIndex :type Integer))
  ;[1 1 1] Door Interaction Code
  (Utilities|Casting|CastToMazeGamePlayerCharacter OtherActor)
  (bind _door_track (Timeline|Open%20Door%20Timeline Reverse)
    (:Update
      (Transformation|SetRelativeRotation (Variables|Default|GetSM_InterativeDoor) (Math|Rotator|MakeRotator 0.0 0.0 (Math|Float|Lerp (Variables|Default|GetClosePosition) (Variables|Default|GetOpenPosition) _door_track)) false false))
    (:Finished
      (Variables|Default|SetIsOpen (not (Variables|Default|GetIsOpen))))))

(event Custom|OpenDoor
  ;[1 1 1] Door Interaction Code
  (bind _door_track (Timeline|Open%20Door%20Timeline Play)
    (:Update
      (Transformation|SetRelativeRotation (Variables|Default|GetSM_InterativeDoor) (Math|Rotator|MakeRotator 0.0 0.0 (Math|Float|Lerp (Variables|Default|GetClosePosition) (Variables|Default|GetOpenPosition) _door_track)) false false))
    (:Finished
      (Variables|Default|SetIsOpen (not (Variables|Default|GetIsOpen))))))

(event EventBeginPlay)

(event Collision|EventActorBeginOverlap
  (params (OtherActor :type Actor%20Object%20Reference)))

(event EventTick
  (params (DeltaSeconds :type Float%20%28single-precision%29)))

(fn ConstructionScript)

(fn Interact
  (params (Interactor :type Maze%20Game%20Player%20Character%20Object%20Reference))
  (if (not (Variables|Default|GetIsOpen))
    (Components|Timeline|SetPlayRate (Variables|Default|GetOpen%20Door%20Timeline) (/ 1.0 (Variables|Default|GetTimeToOpen%28s%29)))
    (CallFunction|OpenDoor)
    (return false)))